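; Level select menu actor with clickable 3D buttons for the tutorial and three levels, plus a Back button that swaps in BP_MainMenu.
; Per-level checkpoint and timer toggles flip a flag and recolor their button blue or red.
; Level buttons open their map, hide the cursor and pass those flags to the GameInstance, preserving the crosshair preference.
; Hovering tutorial or level buttons scales them from sizes cached at BeginPlay.
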(event `self.ReceiveBeginPlay`
  ; Begin play
  (set `self.InitialScaleMainButton` (`SceneComponent.RelativeScale3D` (`self.1`)))
  (set `self.InitialScaleSecondaryButton` (`SceneComponent.RelativeScale3D` (`self.Tuto`))))

(event `self.1.OnClicked`
  (params (TouchedComponent :type "PrimitiveComponent Object Reference") (ButtonPressed :type "Key Structure"))
  (bind _returnvalue (`GameplayStatics.GetPlayerController` 0))
  ; 1
  (`GameplayStatics.OpenLevel` " LEVEL1" true "Game=/Game/FirstPerson/Blueprints/BP_FirstPersonGameMode.BP_FirstPersonGameMode_C")
  (set `PlayerController.bShowMouseCursor` false _returnvalue)
  (set `PlayerController.bEnableClickEvents` false _returnvalue)
  (message `/Game/ProjerUnreal/BP/Interface/BPI_GI.SetCheckpointActivated` (`GameplayStatics.GetGameInstance`) (`self.CheckpointActivatedForLevel1`))
  (bind _hud (message `/Game/ProjerUnreal/BP/Interface/BPI_GI.GetHUDPreferences` (`GameplayStatics.GetGameInstance`)))
  (message `/Game/ProjerUnreal/BP/Interface/BPI_GI.SetHUDPreferences` (`GameplayStatics.GetGameInstance`) (make `/Game/ProjerUnreal/Data/S_HUDPreferences` (break `/Game/ProjerUnreal/Data/S_HUDPreferences` _hud) (`self.TimerActivatedForLevel1`))))

(event `self.Tuto.OnClicked`
  (params (TouchedComponent :type "PrimitiveComponent Object Reference") (ButtonPressed :type "Key Structure"))
  (bind _returnvalue (`GameplayStatics.GetPlayerController` 0))
  ; Tuto
  (`GameplayStatics.OpenLevel` "LD_Blocking" true "Game=/Game/FirstPerson/Blueprints/BP_FirstPersonGameMode.BP_FirstPersonGameMode_C")
  (set `PlayerController.bShowMouseCursor` false _returnvalue)
  (set `PlayerController.bEnableClickEvents` false _returnvalue))

(event `self.Tuto.OnBeginCursorOver`
  (params (TouchedComponent :type "PrimitiveComponent Object Reference"))
  ; Tuto
  (`self.Scale` true TouchedComponent true))

(event `self.1.OnBeginCursorOver`
  (params (TouchedComponent :type "PrimitiveComponent Object Reference"))
  ; 1
  (`self.Scale` true TouchedComponent))

(event `self.Tuto.OnEndCursorOver`
  (params (TouchedComponent :type "PrimitiveComponent Object Reference"))
  ; Tuto
  (`self.Scale` false TouchedComponent true))

(event `self.1.OnEndCursorOver`
  (params (TouchedComponent :type "PrimitiveComponent Object Reference"))
  ; 1
  (`self.Scale` false TouchedComponent))

(event `self.2.OnClicked`
  (params (TouchedComponent :type "PrimitiveComponent Object Reference") (ButtonPressed :type "Key Structure"))
  (bind _returnvalue (`GameplayStatics.GetPlayerController` 0))
  ; 2
  (`GameplayStatics.OpenLevel` " Lucas_Niveau2" true "Game=/Game/FirstPerson/Blueprints/BP_FirstPersonGameMode.BP_FirstPersonGameMode_C")
  (set `PlayerController.bShowMouseCursor` false _returnvalue)
  (set `PlayerController.bEnableClickEvents` false _returnvalue)
  (message `/Game/ProjerUnreal/BP/Interface/BPI_GI.SetCheckpointActivated` (`GameplayStatics.GetGameInstance`) (`self.CheckpointActivatedForLevel2`))
  (bind _hud (message `/Game/ProjerUnreal/BP/Interface/BPI_GI.GetHUDPreferences` (`GameplayStatics.GetGameInstance`)))
  (message `/Game/ProjerUnreal/BP/Interface/BPI_GI.SetHUDPreferences` (`GameplayStatics.GetGameInstance`) (make `/Game/ProjerUnreal/Data/S_HUDPreferences` (break `/Game/ProjerUnreal/Data/S_HUDPreferences` _hud) (`self.TimerActivatedForLevel2`))))

(event `self.2.OnBeginCursorOver`
  (params (TouchedComponent :type "PrimitiveComponent Object Reference"))
  ; 2
  (`self.Scale` true TouchedComponent))

(event `self.2.OnEndCursorOver`
  (params (TouchedComponent :type "PrimitiveComponent Object Reference"))
  ; 2
  (`self.Scale` false TouchedComponent))

(event `self.3.OnClicked`
  (params (TouchedComponent :type "PrimitiveComponent Object Reference") (ButtonPressed :type "Key Structure"))
  (bind _returnvalue (`GameplayStatics.GetPlayerController` 0))
  ; 3
  (`GameplayStatics.OpenLevel` "LD_Blocking_WP" true "Game=/Game/FirstPerson/Blueprints/BP_FirstPersonGameMode.BP_FirstPersonGameMode_C")
  (set `PlayerController.bShowMouseCursor` false _returnvalue)
  (set `PlayerController.bEnableClickEvents` false _returnvalue)
  (message `/Game/ProjerUnreal/BP/Interface/BPI_GI.SetCheckpointActivated` (`GameplayStatics.GetGameInstance`) (`self.CheckpointActivatedForLevel3`))
  (bind _hud (message `/Game/ProjerUnreal/BP/Interface/BPI_GI.GetHUDPreferences` (`GameplayStatics.GetGameInstance`)))
  (message `/Game/ProjerUnreal/BP/Interface/BPI_GI.SetHUDPreferences` (`GameplayStatics.GetGameInstance`) (make `/Game/ProjerUnreal/Data/S_HUDPreferences` (break `/Game/ProjerUnreal/Data/S_HUDPreferences` _hud) (`self.TimerActivatedForLevel3`))))

(event `self.3.OnEndCursorOver`
  (params (TouchedComponent :type "PrimitiveComponent Object Reference"))
  ; 3
  (`self.Scale` false TouchedComponent))

(event `self.3.OnBeginCursorOver`
  (params (TouchedComponent :type "PrimitiveComponent Object Reference"))
  ; 3
  (`self.Scale` true TouchedComponent))

(event `self.1_Checkpoint.OnClicked`
  (params (TouchedComponent :type "PrimitiveComponent Object Reference") (ButtonPressed :type "Key Structure"))
  ; No checkpoint button
  (bind _isa (`/Engine/EditorBlueprintResources/StandardMacros.FlipFlop`)
    (:`A`
      _)
    (:`B`
      _))
  (bind _output_get (set `self.CheckpointActivatedForLevel1` _isa))
  (if _output_get
    (`PrimitiveComponent.SetMaterial` (`self.1_Checkpoint`) 0 "/Game/ProjerUnreal/Materials/M_Blue.M_Blue")
    (else
      (`PrimitiveComponent.SetMaterial` (`self.1_Checkpoint`) 0 "/Game/ProjerUnreal/Materials/M_Red.M_Red"))))

(event `self.1_Timer.OnClicked`
  (params (TouchedComponent :type "PrimitiveComponent Object Reference") (ButtonPressed :type "Key Structure"))
  (bind _1_timer (`self.1_Timer`))
  ; Timer button
  (bind _isa (`/Engine/EditorBlueprintResources/StandardMacros.FlipFlop`)
    (:`A`
      _)
    (:`B`
      _))
  (bind _output_get (set `self.TimerActivatedForLevel1` _isa))
  (if _output_get
    (`PrimitiveComponent.SetMaterial` _1_timer 0 "/Game/ProjerUnreal/Materials/M_Blue.M_Blue")
    (else
      (`PrimitiveComponent.SetMaterial` _1_timer 0 "/Game/ProjerUnreal/Materials/M_Red.M_Red"))))

(event `self.2_Checkpoint.OnClicked`
  (params (TouchedComponent :type "PrimitiveComponent Object Reference") (ButtonPressed :type "Key Structure"))
  (bind _2_checkpoint (`self.2_Checkpoint`))
  ; No checkpoint button
  (bind _isa (`/Engine/EditorBlueprintResources/StandardMacros.FlipFlop`)
    (:`A`
      _)
    (:`B`
      _))
  (bind _output_get (set `self.CheckpointActivatedForLevel2` _isa))
  (if _output_get
    (`PrimitiveComponent.SetMaterial` _2_checkpoint 0 "/Game/ProjerUnreal/Materials/M_Blue.M_Blue")
    (else
      (`PrimitiveComponent.SetMaterial` _2_checkpoint 0 "/Game/ProjerUnreal/Materials/M_Red.M_Red"))))

(event `self.2_Timer.OnClicked`
  (params (TouchedComponent :type "PrimitiveComponent Object Reference") (ButtonPressed :type "Key Structure"))
  (bind _2_timer (`self.2_Timer`))
  ; Timer button
  (bind _isa (`/Engine/EditorBlueprintResources/StandardMacros.FlipFlop`)
    (:`A`
      _)
    (:`B`
      _))
  (bind _output_get (set `self.TimerActivatedForLevel2` _isa))
  (if _output_get
    (`PrimitiveComponent.SetMaterial` _2_timer 0 "/Game/ProjerUnreal/Materials/M_Blue.M_Blue")
    (else
      (`PrimitiveComponent.SetMaterial` _2_timer 0 "/Game/ProjerUnreal/Materials/M_Red.M_Red"))))

(event `self.3_Checkpoint.OnClicked`
  (params (TouchedComponent :type "PrimitiveComponent Object Reference") (ButtonPressed :type "Key Structure"))
  (bind _3_checkpoint (`self.3_Checkpoint`))
  ; No checkpoint button
  (bind _isa (`/Engine/EditorBlueprintResources/StandardMacros.FlipFlop`)
    (:`A`
      _)
    (:`B`
      _))
  (bind _output_get (set `self.CheckpointActivatedForLevel3` _isa))
  (if _output_get
    (`PrimitiveComponent.SetMaterial` _3_checkpoint 0 "/Game/ProjerUnreal/Materials/M_Blue.M_Blue")
    (else
      (`PrimitiveComponent.SetMaterial` _3_checkpoint 0 "/Game/ProjerUnreal/Materials/M_Red.M_Red"))))

(event `self.3_Timer.OnClicked`
  (params (TouchedComponent :type "PrimitiveComponent Object Reference") (ButtonPressed :type "Key Structure"))
  (bind _3_timer (`self.3_Timer`))
  ; Timer button
  (bind _isa (`/Engine/EditorBlueprintResources/StandardMacros.FlipFlop`)
    (:`A`
      _)
    (:`B`
      _))
  (bind _output_get (set `self.TimerActivatedForLevel3` _isa))
  (if _output_get
    (`PrimitiveComponent.SetMaterial` _3_timer 0 "/Game/ProjerUnreal/Materials/M_Blue.M_Blue")
    (else
      (`PrimitiveComponent.SetMaterial` _3_timer 0 "/Game/ProjerUnreal/Materials/M_Red.M_Red"))))

(event `self.Back1.OnClicked`
  (params (TouchedComponent :type "PrimitiveComponent Object Reference") (ButtonPressed :type "Key Structure"))
  (`|SpawnActorFromClass` "/Game/ProjerUnreal/BP/Menu/BP_MainMenu.BP_MainMenu_C" (`SceneComponent.K2_GetComponentToWorld` (`self.DefaultSceneRoot`)) "Undefined" "MultiplyWithRoot" null null)
  (`self.K2_DestroyActor`))

(fn `ActiveMenu`
  (params (Panel :type "/Game/ProjerUnreal/Data/E_MenuPanel Enum" :default "NewEnumerator0")))

(fn `Scale`
  (params (Extend :type Boolean) (Target :type "SceneComponent Object Reference") (SecondarySize :type Boolean))
  (if SecondarySize
    (if Extend
      (`SceneComponent.SetRelativeScale3D` Target (* (`self.InitialScaleSecondaryButton`) (`self.ScaleMultiplier`)))
      (else
        (`SceneComponent.SetRelativeScale3D` Target (`self.InitialScaleSecondaryButton`))))
    (elif Extend
      (`SceneComponent.SetRelativeScale3D` Target (* (`self.InitialScaleMainButton`) (`self.ScaleMultiplier`)))
      (else
        (`SceneComponent.SetRelativeScale3D` Target (`self.InitialScaleMainButton`))))))

(fn `UserConstructionScript`)