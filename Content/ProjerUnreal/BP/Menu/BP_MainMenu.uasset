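; BP_MainMenu is a 3D main menu actor with clickable Play, Options, Quit and Save components.
; Play opens the GymDim level with the first-person game mode and disables cursor input, Quit exits, and Save calls SaveGameMessage on the game instance.
; Options replaces this actor with a spawned BP_OptionsMenu at the same transform.
; Hovering Play, Options or Quit enlarges it through Scale, based on Play's initial scale.
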(event `self.ReceiveBeginPlay`
  ; Begin play
  (set `self.InitialScaleMainButton` (`SceneComponent.RelativeScale3D` (`self.Play`))))

(event `self.Play.OnClicked`
  (params (TouchedComponent :type "PrimitiveComponent Object Reference") (ButtonPressed :type "Key Structure"))
  (bind _returnvalue (`GameplayStatics.GetPlayerController` 0))
  ; Play Panel
  (`GameplayStatics.OpenLevel` "GymDim" true "Game=/Game/FirstPerson/Blueprints/BP_FirstPersonGameMode.BP_FirstPersonGameMode_C")
  (set `PlayerController.bShowMouseCursor` false _returnvalue)
  (set `PlayerController.bEnableClickEvents` false _returnvalue))

(event `self.Play.OnBeginCursorOver`
  (params (TouchedComponent :type "PrimitiveComponent Object Reference"))
  ; Play Panel
  (`self.Scale` true TouchedComponent))

(event `self.Play.OnEndCursorOver`
  (params (TouchedComponent :type "PrimitiveComponent Object Reference"))
  ; Play Panel
  (`self.Scale` false TouchedComponent))

(event `self.Quit.OnClicked`
  (params (TouchedComponent :type "PrimitiveComponent Object Reference") (ButtonPressed :type "Key Structure"))
  ; Quit panel
  (`KismetSystemLibrary.QuitGame` (`GameplayStatics.GetPlayerController` 0) "Quit"))

(event `self.Quit.OnBeginCursorOver`
  (params (TouchedComponent :type "PrimitiveComponent Object Reference"))
  ; Quit panel
  (`self.Scale` true TouchedComponent))

(event `self.Quit.OnEndCursorOver`
  (params (TouchedComponent :type "PrimitiveComponent Object Reference"))
  ; Quit panel
  (`self.Scale` false TouchedComponent))

(event `self.Options.OnClicked`
  (params (TouchedComponent :type "PrimitiveComponent Object Reference") (ButtonPressed :type "Key Structure"))
  ; Options panel
  (`|SpawnActorFromClass` "/Game/ProjerUnreal/BP/Menu/BP_OptionsMenu.BP_OptionsMenu_C" (`SceneComponent.K2_GetComponentToWorld` (`self.DefaultSceneRoot`)) "Undefined" "MultiplyWithRoot" null null)
  (`self.K2_DestroyActor`))

(event `self.Options.OnBeginCursorOver`
  (params (TouchedComponent :type "PrimitiveComponent Object Reference"))
  ; Options panel
  (`self.Scale` true TouchedComponent))

(event `self.Options.OnEndCursorOver`
  (params (TouchedComponent :type "PrimitiveComponent Object Reference"))
  ; Options panel
  (`self.Scale` false TouchedComponent))

(event `self.Save.OnClicked`
  (params (TouchedComponent :type "PrimitiveComponent Object Reference") (ButtonPressed :type "Key Structure"))
  (message `/Game/ProjerUnreal/BP/Interface/BPI_GI.SaveGame` (`GameplayStatics.GetGameInstance`)))

(fn `ActiveMenu`
  (params (Panel :type "/Game/ProjerUnreal/Data/E_MenuPanel Enum" :default "NewEnumerator0")))

(fn `Scale`
  (params (Extend :type Boolean) (Target :type "SceneComponent Object Reference"))
  (if Extend
    (`SceneComponent.SetRelativeScale3D` Target (* (`self.InitialScaleMainButton`) (`self.ScaleMultiplier`)))
    (else
      (`SceneComponent.SetRelativeScale3D` Target (`self.InitialScaleMainButton`)))))

(fn `UserConstructionScript`)