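; BP_OptionsMenu is an in-world options menu actor with clickable components for Input, HUD, Sound and Back.
; Each click spawns the matching menu actor (input, HUD, sound or main menu) at the root transform, then destroys this actor.
; Hovering Input, HUD or Sound enlarges it by a multiplier of the Input button's scale cached on BeginPlay; Back has no hover effect.
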(event `self.ReceiveBeginPlay`
  ; Begin play
  (set `self.InitialScaleMainButton` (`SceneComponent.RelativeScale3D` (`self.Input`))))

(event `self.Input.OnClicked`
  (params (TouchedComponent :type "PrimitiveComponent Object Reference") (ButtonPressed :type "Key Structure"))
  ; Input - Open Input Menu
  (`|SpawnActorFromClass` "/Game/ProjerUnreal/BP/Menu/BP_InputMenu.BP_InputMenu_C" (`SceneComponent.K2_GetComponentToWorld` (`self.DefaultSceneRoot`)) "Undefined" "MultiplyWithRoot" null null)
  (`self.K2_DestroyActor`))

(event `self.Back1.OnClicked`
  (params (TouchedComponent :type "PrimitiveComponent Object Reference") (ButtonPressed :type "Key Structure"))
  (`|SpawnActorFromClass` "/Game/ProjerUnreal/BP/Menu/BP_MainMenu.BP_MainMenu_C" (`SceneComponent.K2_GetComponentToWorld` (`self.DefaultSceneRoot`)) "Undefined" "MultiplyWithRoot" null null)
  (`self.K2_DestroyActor`))

(event `self.Input.OnBeginCursorOver`
  (params (TouchedComponent :type "PrimitiveComponent Object Reference"))
  ; Input - Open Input Menu
  (`self.Scale` true TouchedComponent))

(event `self.Input.OnEndCursorOver`
  (params (TouchedComponent :type "PrimitiveComponent Object Reference"))
  ; Input - Open Input Menu
  (`self.Scale` false TouchedComponent))

(event `self.HUD.OnClicked`
  (params (TouchedComponent :type "PrimitiveComponent Object Reference") (ButtonPressed :type "Key Structure"))
  ; HUD - Open HUD menu
  (`|SpawnActorFromClass` "/Game/ProjerUnreal/BP/Menu/BP_HUDMenu.BP_HUDMenu_C" (`SceneComponent.K2_GetComponentToWorld` (`self.DefaultSceneRoot`)) "Undefined" "MultiplyWithRoot" null null)
  (`self.K2_DestroyActor`))

(event `self.HUD.OnBeginCursorOver`
  (params (TouchedComponent :type "PrimitiveComponent Object Reference"))
  ; HUD - Open HUD menu
  (`self.Scale` true TouchedComponent))

(event `self.HUD.OnEndCursorOver`
  (params (TouchedComponent :type "PrimitiveComponent Object Reference"))
  ; HUD - Open HUD menu
  (`self.Scale` false TouchedComponent))

(event `self.Sound.OnClicked`
  (params (TouchedComponent :type "PrimitiveComponent Object Reference") (ButtonPressed :type "Key Structure"))
  ; Sound - Open sound menu
  (`|SpawnActorFromClass` "/Game/ProjerUnreal/BP/Menu/BP_SoundMenu.BP_SoundMenu_C" (`SceneComponent.K2_GetComponentToWorld` (`self.DefaultSceneRoot`)) "Undefined" "MultiplyWithRoot" null null)
  (`self.K2_DestroyActor`))

(event `self.Sound.OnBeginCursorOver`
  (params (TouchedComponent :type "PrimitiveComponent Object Reference"))
  ; Sound - Open sound menu
  (`self.Scale` true TouchedComponent))

(event `self.Sound.OnEndCursorOver`
  (params (TouchedComponent :type "PrimitiveComponent Object Reference"))
  ; Sound - Open sound menu
  (`self.Scale` false TouchedComponent))

(fn `ActiveMenu`
  (params (Panel :type "/Game/ProjerUnreal/Data/E_MenuPanel Enum" :default "NewEnumerator0")))

(fn `Scale`
  (params (Extend :type Boolean) (Target :type "SceneComponent Object Reference"))
  (if Extend
    (`SceneComponent.SetRelativeScale3D` Target (* (`self.InitialScaleMainButton`) (`self.ScaleMultiplier`)))
    (else
      (`SceneComponent.SetRelativeScale3D` Target (`self.InitialScaleMainButton`)))))

(fn `UserConstructionScript`)