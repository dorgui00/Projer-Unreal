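; BP_InputMenu is a 3D menu actor that shows input key bindings, with a Back button that spawns BP_OptionsMenu and destroys this one.
; Four text and WBP_KeyBind rows act as a sliding window over InputName and Enhanced Input mappings, paired by index.
; BP_MenuPawn scroll events shift the window within list bounds, and BeginPlay retries each tick until mappings exist.
; Hovering an input zone scales it up.
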(event `self.ReceiveBeginPlay`
  (set `self.InitialScaleMainButton` (`SceneComponent.RelativeScale3D` (`self.InputZone4`)))
  (`KismetArrayLibrary.Array_Add` (`self.TextZone`) (`self.Input1Text`))
  (`KismetArrayLibrary.Array_Add` (`self.TextZone`) (`self.Input2Text`))
  (`KismetArrayLibrary.Array_Add` (`self.TextZone`) (`self.Input3Text`))
  (`KismetArrayLibrary.Array_Add` (`self.TextZone`) (`self.Input4Text`))
  (bind _aswbp_key_bind (cast `/Game/ProjerUnreal/BP/Menu/WBP_KeyBind` (`WidgetComponent.GetWidget` (`self.Widget1`))))
  (`KismetArrayLibrary.Array_Add` (`self.KeyZone`) _aswbp_key_bind)
  (bind _aswbp_key_bind_2 (cast `/Game/ProjerUnreal/BP/Menu/WBP_KeyBind` (`WidgetComponent.GetWidget` (`self.Widget2`))))
  (`KismetArrayLibrary.Array_Add` (`self.KeyZone`) _aswbp_key_bind_2)
  (bind _aswbp_key_bind_3 (cast `/Game/ProjerUnreal/BP/Menu/WBP_KeyBind` (`WidgetComponent.GetWidget` (`self.Widget3`))))
  (`KismetArrayLibrary.Array_Add` (`self.KeyZone`) _aswbp_key_bind_3)
  (bind _aswbp_key_bind_4 (cast `/Game/ProjerUnreal/BP/Menu/WBP_KeyBind` (`WidgetComponent.GetWidget` (`self.Widget4`))))
  (`KismetArrayLibrary.Array_Add` (`self.KeyZone`) _aswbp_key_bind_4)
  (bind _asbp_menu_pawn (cast `/Game/ProjerUnreal/BP/Character/BP_MenuPawn` (`GameplayStatics.GetPlayerPawn` 0)))
  (add `/Game/ProjerUnreal/BP/Character/BP_MenuPawn.ED_ScrollUp` _asbp_menu_pawn (`|CreateDelegate` :!event `CE_ScrollUp`))
  (add `/Game/ProjerUnreal/BP/Character/BP_MenuPawn.ED_ScrollDown` _asbp_menu_pawn (`|CreateDelegate` :!event `CE_ScrollDown`))
  (bind _output_get (set `self.Mappings` (`EnhancedInputSubsystemInterface.GetAllPlayerMappableActionKeyMappings` (pcsubsystem `EnhancedInputLocalPlayerSubsystem` (`GameplayStatics.GetPlayerController` 0)))))
  (if (`KismetMathLibrary.Conv_IntToBool` (`KismetArrayLibrary.Array_Length` _output_get)) :!label _label
    (`self.CE_LoadInputText`)
    (else
      (`KismetSystemLibrary.DelayUntilNextTick`)
      (goto _label))))

(event `self.Back1.OnClicked`
  (params (TouchedComponent :type "PrimitiveComponent Object Reference") (ButtonPressed :type "Key Structure"))
  ; Back - Open OptionsMenu
  (`|SpawnActorFromClass` "/Game/ProjerUnreal/BP/Menu/BP_OptionsMenu.BP_OptionsMenu_C" (`SceneComponent.K2_GetComponentToWorld` (`self.DefaultSceneRoot`)) "Undefined" "MultiplyWithRoot" null null)
  (`self.K2_DestroyActor`))

(event `CE_ScrollDown`
  (if (<= (+ (`self.Index`) 4) (- (`KismetArrayLibrary.Array_Length` (`self.InputName`)) 1))
    (`/Engine/EditorBlueprintResources/StandardMacros.IncrementInt` (`self.Index`)
      (:`  `
        (`self.CE_LoadInputText`)))))

(event `CE_ScrollUp`
  (if (>= (- (`self.Index`) 1) 0)
    (`/Engine/EditorBlueprintResources/StandardMacros.DecrementInt` (`self.Index`)
      (:`  `
        (`self.CE_LoadInputText`)))))

(event `CE_SetKeyBind`
  (params (`Mapping Name` :type Name))
  (for (_array_element _array_index) (`self.KeyZone`)
    (bind _returnvalue (+ _array_index (`self.Index`)))
    (bind (_output_triggers _output_modifiers _output_action _output_key) (break `EnhancedActionKeyMapping` (`|GetArrayItem` (`self.Mappings`) _returnvalue)))
    (bind _output_inputname (break `/Game/ProjerUnreal/Data/S_InputData` (`|GetArrayItem` (`self.InputName`) _returnvalue)))
    (`/Game/ProjerUnreal/BP/Menu/WBP_KeyBind.CE_SetValue` _array_element _output_key (`KismetStringLibrary.Conv_StringToName` _output_inputname))))

(event `CE_LoadInputText`
  (for (_array_element _array_index) (`self.TextZone`)
    (bind _output_inputname (break `/Game/ProjerUnreal/Data/S_InputData` (`|GetArrayItem` (`self.InputName`) (+ _array_index (`self.Index`)))))
    (`TextRenderComponent.K2_SetText` _array_element (`KismetTextLibrary.Conv_StringToText` _output_inputname)))
  (`self.CE_SetKeyBind` "None"))

(event `self.InputZone1.OnBeginCursorOver`
  (params (TouchedComponent :type "PrimitiveComponent Object Reference"))
  (`self.Scale` true TouchedComponent))

(event `self.InputZone2.OnBeginCursorOver`
  (params (TouchedComponent :type "PrimitiveComponent Object Reference"))
  (`self.Scale` true TouchedComponent))

(event `self.InputZone3.OnBeginCursorOver`
  (params (TouchedComponent :type "PrimitiveComponent Object Reference"))
  (`self.Scale` true TouchedComponent))

(event `self.InputZone4.OnBeginCursorOver`
  (params (TouchedComponent :type "PrimitiveComponent Object Reference"))
  (`self.Scale` true TouchedComponent))

(event `self.InputZone1.OnEndCursorOver`
  (params (TouchedComponent :type "PrimitiveComponent Object Reference"))
  (`self.Scale` false TouchedComponent))

(event `self.InputZone2.OnEndCursorOver`
  (params (TouchedComponent :type "PrimitiveComponent Object Reference"))
  (`self.Scale` false TouchedComponent))

(event `self.InputZone3.OnEndCursorOver`
  (params (TouchedComponent :type "PrimitiveComponent Object Reference"))
  (`self.Scale` false TouchedComponent))

(event `self.InputZone4.OnEndCursorOver`
  (params (TouchedComponent :type "PrimitiveComponent Object Reference"))
  (`self.Scale` false TouchedComponent))

(fn `ActiveMenu`
  (params (Panel :type "/Game/ProjerUnreal/Data/E_MenuPanel Enum" :default "NewEnumerator0")))

(fn `Scale`
  (params (Extend :type Boolean) (Target :type "SceneComponent Object Reference"))
  (if Extend
    (`SceneComponent.SetRelativeScale3D` Target (* (`self.InitialScaleMainButton`) (`self.ScaleMultiplier`)))
    (else
      (`SceneComponent.SetRelativeScale3D` Target (`self.InitialScaleMainButton`)))))

(fn `UserConstructionScript`)