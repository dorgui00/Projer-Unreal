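; BP_SoundMenu is an in-world sound settings menu actor with clickable Ambient, Music, Effect and Back components.
; Each category click creates a WBP_SoundBar widget for that sound class and adds it to the viewport.
; Hover scales category buttons through Scale, using Ambient's initial scale as the shared base.
; Back spawns BP_OptionsMenu at the root's transform and destroys this actor; ActiveMenu is an empty stub.
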(event `self.ReceiveBeginPlay`
  ; Begin play
  (set `self.InitialScaleMainButton` (`SceneComponent.RelativeScale3D` (`self.Ambient`))))

(event `self.Ambient.OnBeginCursorOver`
  (params (TouchedComponent :type "PrimitiveComponent Object Reference"))
  ; Visual
  (`self.Scale` true TouchedComponent))

(event `self.Ambient.OnClicked`
  (params (TouchedComponent :type "PrimitiveComponent Object Reference") (ButtonPressed :type "Key Structure"))
  (bind _returnvalue (`|CreateWidget` "/Game/ProjerUnreal/BP/Menu/WBP_SoundBar.WBP_SoundBar_C"))
  (bind _output_get (set `self.SoundBar` _returnvalue))
  (`UserWidget.AddToViewport` _output_get 0))

(event `self.Ambient.OnEndCursorOver`
  (params (TouchedComponent :type "PrimitiveComponent Object Reference"))
  ; Visual
  (`self.Scale` false TouchedComponent))

(event `self.Music.OnClicked`
  (params (TouchedComponent :type "PrimitiveComponent Object Reference") (ButtonPressed :type "Key Structure"))
  (bind _returnvalue (`|CreateWidget` "/Game/ProjerUnreal/BP/Menu/WBP_SoundBar.WBP_SoundBar_C" null "NewEnumerator2"))
  (bind _output_get (set `self.SoundBar` _returnvalue))
  (`UserWidget.AddToViewport` _output_get 0))

(event `self.Music.OnBeginCursorOver`
  (params (TouchedComponent :type "PrimitiveComponent Object Reference"))
  ; Visual
  (`self.Scale` true TouchedComponent))

(event `self.Effect.OnClicked`
  (params (TouchedComponent :type "PrimitiveComponent Object Reference") (ButtonPressed :type "Key Structure"))
  (bind _returnvalue (`|CreateWidget` "/Game/ProjerUnreal/BP/Menu/WBP_SoundBar.WBP_SoundBar_C" null "NewEnumerator1"))
  (bind _output_get (set `self.SoundBar` _returnvalue))
  (`UserWidget.AddToViewport` _output_get 0))

(event `self.Music.OnEndCursorOver`
  (params (TouchedComponent :type "PrimitiveComponent Object Reference"))
  ; Visual
  (`self.Scale` false TouchedComponent))

(event `self.Effect.OnBeginCursorOver`
  (params (TouchedComponent :type "PrimitiveComponent Object Reference"))
  ; Visual
  (`self.Scale` true TouchedComponent))

(event `self.Back.OnClicked`
  (params (TouchedComponent :type "PrimitiveComponent Object Reference") (ButtonPressed :type "Key Structure"))
  (`|SpawnActorFromClass` "/Game/ProjerUnreal/BP/Menu/BP_OptionsMenu.BP_OptionsMenu_C" (`SceneComponent.K2_GetComponentToWorld` (`self.DefaultSceneRoot`)) "Undefined" "MultiplyWithRoot" null null)
  (`self.K2_DestroyActor`))

(event `self.Effect.OnEndCursorOver`
  (params (TouchedComponent :type "PrimitiveComponent Object Reference"))
  ; Visual
  (`self.Scale` false TouchedComponent))

(fn `ActiveMenu`
  (params (Panel :type "/Game/ProjerUnreal/Data/E_MenuPanel Enum" :default "NewEnumerator0")))

(fn `Scale`
  (params (Extend :type Boolean) (Target :type "SceneComponent Object Reference"))
  (if Extend
    (`SceneComponent.SetRelativeScale3D` Target (* (`self.InitialScaleMainButton`) (`self.ScaleMultiplier`)))
    (else
      (`SceneComponent.SetRelativeScale3D` Target (`self.InitialScaleMainButton`)))))

(fn `UserConstructionScript`)