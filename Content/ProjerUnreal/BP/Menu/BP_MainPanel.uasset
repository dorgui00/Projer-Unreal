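; BP_MainPanel is an actor that sets up the game's main menu in the world.
; On BeginPlay it enables the mouse cursor, click and mouse-over events on player 0, then spawns BP_MainMenu at the MenuParent component's world transform.
; The Scale function sets a target's relative scale to zero in both branches, and ActiveMenu is an empty stub; neither is called here.
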(event `self.ReceiveBeginPlay`
  (bind _returnvalue (`GameplayStatics.GetPlayerController` 0))
  (set `PlayerController.bShowMouseCursor` true _returnvalue)
  (set `PlayerController.bEnableClickEvents` true _returnvalue)
  (set `PlayerController.bEnableMouseOverEvents` true _returnvalue)
  (`|SpawnActorFromClass` "/Game/ProjerUnreal/BP/Menu/BP_MainMenu.BP_MainMenu_C" (`SceneComponent.K2_GetComponentToWorld` (`self.MenuParent`)) "Undefined" "MultiplyWithRoot" null null))

(fn `ActiveMenu`
  (params (Panel :type "/Game/ProjerUnreal/Data/E_MenuPanel Enum" :default "NewEnumerator0")))

(fn `Scale`
  (params (Extend :type Boolean) (Target :type "SceneComponent Object Reference"))
  (if Extend
    (`SceneComponent.SetRelativeScale3D` Target (* (0.0 0.0 0.0) (0.0 0.0 0.0)))
    (else
      (`SceneComponent.SetRelativeScale3D` Target (0.0 0.0 0.0)))))

(fn `UserConstructionScript`)