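; BP_HUDMenu is a 3D menu actor for toggling the crosshair and timer HUD preferences.
; Clicks flip the values stored through the GameInstance and swap button materials between blue and red, which the construction script also sets from saved preferences.
; Quality opens a WBP_Quality widget with a close binding, while Back spawns BP_OptionsMenu and destroys this actor.
; A Scale helper is defined but not called here, and ActiveMenu is empty.
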(event `self.ReceiveBeginPlay`
  (set `self.InitialScaleMainButton` (`SceneComponent.RelativeScale3D` (`self.InputZone4`))))

(event `self.Back1.OnClicked`
  (params (TouchedComponent :type "PrimitiveComponent Object Reference") (ButtonPressed :type "Key Structure"))
  ; Back - Open OptionsMenu
  (`|SpawnActorFromClass` "/Game/ProjerUnreal/BP/Menu/BP_OptionsMenu.BP_OptionsMenu_C" (`SceneComponent.K2_GetComponentToWorld` (`self.DefaultSceneRoot`)) "Undefined" "MultiplyWithRoot" null null)
  (`self.K2_DestroyActor`))

(event `self.CrossairInput.OnClicked`
  (params (TouchedComponent :type "PrimitiveComponent Object Reference") (ButtonPressed :type "Key Structure"))
  (bind _hud (message `/Game/ProjerUnreal/BP/Interface/BPI_GI.GetHUDPreferences` (`GameplayStatics.GetGameInstance`)))
  (bind _returnvalue (not (break `/Game/ProjerUnreal/Data/S_HUDPreferences` _hud)))
  (message `/Game/ProjerUnreal/BP/Interface/BPI_GI.SetHUDPreferences` (`GameplayStatics.GetGameInstance`) (make `/Game/ProjerUnreal/Data/S_HUDPreferences` _returnvalue (`.Timer_3_F85C7C41433EF129E3D1C1A60CCF42B6` (break `/Game/ProjerUnreal/Data/S_HUDPreferences` _hud))))
  (if _returnvalue
    (`PrimitiveComponent.SetMaterial` (`self.CrossairInput`) 0 "/Game/ProjerUnreal/Materials/M_Blue.M_Blue")
    (else
      (`PrimitiveComponent.SetMaterial` (`self.CrossairInput`) 0 "/Game/ProjerUnreal/Materials/M_Red.M_Red"))))

(event `self.TimerInput.OnClicked`
  (params (TouchedComponent :type "PrimitiveComponent Object Reference") (ButtonPressed :type "Key Structure"))
  (bind _hud (message `/Game/ProjerUnreal/BP/Interface/BPI_GI.GetHUDPreferences` (`GameplayStatics.GetGameInstance`)))
  (bind _returnvalue (not (`.Timer_3_F85C7C41433EF129E3D1C1A60CCF42B6` (break `/Game/ProjerUnreal/Data/S_HUDPreferences` _hud))))
  (message `/Game/ProjerUnreal/BP/Interface/BPI_GI.SetHUDPreferences` (`GameplayStatics.GetGameInstance`) (make `/Game/ProjerUnreal/Data/S_HUDPreferences` (break `/Game/ProjerUnreal/Data/S_HUDPreferences` _hud) _returnvalue))
  (if _returnvalue
    (`PrimitiveComponent.SetMaterial` (`self.TimerInput`) 0 "/Game/ProjerUnreal/Materials/M_Blue.M_Blue")
    (else
      (`PrimitiveComponent.SetMaterial` (`self.TimerInput`) 0 "/Game/ProjerUnreal/Materials/M_Red.M_Red"))))

(event `self.Quality.OnClicked`
  (params (TouchedComponent :type "PrimitiveComponent Object Reference") (ButtonPressed :type "Key Structure"))
  (bind _returnvalue (`|CreateWidget` "/Game/ProjerUnreal/BP/Menu/WBP_Quality.WBP_Quality_C"))
  (bind _output_get (set `self.QualityMenu` _returnvalue))
  (`UserWidget.AddToViewport` _output_get 0)
  (add `Button.OnClicked` (`/Game/ProjerUnreal/BP/Menu/WBP_Quality.Button_Close` (`self.QualityMenu`)) (delegate `OnClicked_Event`)))

(event `OnClicked_Event`
  (`Widget.RemoveFromParent` (`self.QualityMenu`)))

(fn `ActiveMenu`
  (params (Panel :type "/Game/ProjerUnreal/Data/E_MenuPanel Enum" :default "NewEnumerator0")))

(fn `Scale`
  (params (Extend :type Boolean) (Target :type "SceneComponent Object Reference"))
  (if Extend
    (`SceneComponent.SetRelativeScale3D` Target (* (`self.InitialScaleMainButton`) (`self.ScaleMultiplier`)))
    (else
      (`SceneComponent.SetRelativeScale3D` Target (`self.InitialScaleMainButton`)))))

(fn `UserConstructionScript`
  (bind _hud (message `/Game/ProjerUnreal/BP/Interface/BPI_GI.GetHUDPreferences` (`GameplayStatics.GetGameInstance`)))
  (if (break `/Game/ProjerUnreal/Data/S_HUDPreferences` _hud)
    (`PrimitiveComponent.SetMaterial` (`self.CrossairInput`) 0 "/Game/ProjerUnreal/Materials/M_Blue.M_Blue")
    (else
      (`PrimitiveComponent.SetMaterial` (`self.CrossairInput`) 0 "/Game/ProjerUnreal/Materials/M_Red.M_Red")))
  (if (`.Timer_3_F85C7C41433EF129E3D1C1A60CCF42B6` (break `/Game/ProjerUnreal/Data/S_HUDPreferences` _hud))
    (`PrimitiveComponent.SetMaterial` (`self.TimerInput`) 0 "/Game/ProjerUnreal/Materials/M_Blue.M_Blue")
    (else
      (`PrimitiveComponent.SetMaterial` (`self.TimerInput`) 0 "/Game/ProjerUnreal/Materials/M_Red.M_Red"))))