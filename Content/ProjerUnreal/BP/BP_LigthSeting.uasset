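; Spotlight Blueprint that changes its brightness with the current dimension, future or past.
; BeginPlay binds to the dimension-swap dispatcher on GI_Main, then applies color, cone angles and source shape from variables to the SpotLight.
; The LateNuis event reads the dimension from the game instance and sets the future or past intensity.
; Intensity is only set in that event, not at BeginPlay.
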(event `self.ReceiveBeginPlay`
  (bind _asgi_main (cast `/Game/ProjerUnreal/BP/System/GI_Main` (`GameplayStatics.GetGameInstance`)))
  (add `/Game/ProjerUnreal/BP/System/GI_Main.ED_SwapDimension` _asgi_main (`|CreateDelegate` :!event `LateNuis`))
  (`LightComponent.SetLightColor` (`self.SpotLight`) (`self.New Light Color`) true)
  (`SpotLightComponent.SetInnerConeAngle` (`self.SpotLight`) (`self.New Inner Cone Angle`))
  (`SpotLightComponent.SetOuterConeAngle` (`self.SpotLight`) (`self.New Outer Cone Angle`))
  (`PointLightComponent.SetSourceRadius` (`self.SpotLight`) (`self.New Source Radius`))
  (`PointLightComponent.SetSoftSourceRadius` (`self.SpotLight`) (`self.New Soft Source Radius`))
  (`PointLightComponent.SetSourceLength` (`self.SpotLight`) (`self.New Source Length`)))

(event `LateNuis`
  (bind _dimension (message `/Game/ProjerUnreal/BP/Interface/BPI_GI.GetDimension` (`GameplayStatics.GetGameInstance`)))
  (if (`|EnumEquality` _dimension "NewEnumerator1")
    (`LightComponent.SetIntensity` (`self.SpotLight`) (`self.New IntensityFutur`))
    (else
      (`LightComponent.SetIntensity` (`self.SpotLight`) (`self.New IntensityPasser`)))))

(fn `UserConstructionScript`)