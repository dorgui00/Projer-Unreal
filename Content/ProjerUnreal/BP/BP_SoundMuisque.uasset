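; BP_SoundMuisque is a music/sound actor that switches audio between future and past dimensions.
; On BeginPlay it assigns sounds and shared attenuation to two audio components, binds to GI_Main's dimension-swap dispatcher, and starts both playing together.
; Its Activet event queries the current dimension from the game instance and sets one track to full volume and the other near-silent, so both keep running rather than restarting.
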(event `self.ReceiveBeginPlay`
  (`AudioComponent.SetSound` (`self.SoudsFutur`) (`self.New SoundFutur`))
  (`AudioComponent.SetSound` (`self.SoudsPaser`) (`self.New SoundPasser`))
  (set `AudioComponent.AttenuationSettings` (`self.Attenuation Settings`) (`self.SoudsFutur`))
  (set `AudioComponent.AttenuationSettings` (`self.Attenuation Settings`) (`self.SoudsPaser`))
  (bind _asgi_main (cast `/Game/ProjerUnreal/BP/GI_Main` (`GameplayStatics.GetGameInstance`)))
  (add `/Game/ProjerUnreal/BP/GI_Main.ED_SwapDimension` _asgi_main (`|CreateDelegate` :!event `Activet`))
  (`AudioComponent.Play` (`self.SoudsFutur`) 0.0)
  (`AudioComponent.Play` (`self.SoudsPaser`) 0.0))

(event `self.Activet`
  (bind _soudspaser (`self.SoudsPaser`))
  (bind _soudsfutur (`self.SoudsFutur`))
  (bind _dimension (message `/Game/ProjerUnreal/BP/Interface/BPI_GI.GetDimension` (`GameplayStatics.GetGameInstance`)))
  (if (`|EnumEquality` _dimension "NewEnumerator1")
    (`AudioComponent.SetVolumeMultiplier` _soudspaser 0.001)
    (`AudioComponent.SetVolumeMultiplier` _soudsfutur 1.0)
    (else
      (`AudioComponent.SetVolumeMultiplier` _soudsfutur 0.001)
      (`AudioComponent.SetVolumeMultiplier` _soudspaser 1.0))))

(fn `UserConstructionScript`)