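; BP_Wallrun is a world object for a wall-run surface, built around a plane mesh and two arrow components.
; Its events set the plane's material and switch its collision between query-and-physics and none to activate or disable it.
; Getter functions expose Arrow and ArrowRight to other code, and the construction script only calls the parent.
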(event `/Game/ProjerUnreal/BP/Interface/BPI_DimensionObject.SetMaterial`
  (params (Mat :type "MaterialInstance Object Reference"))
  (`PrimitiveComponent.SetMaterial` (`self.Plane`) 0 Mat))

(event `/Game/ProjerUnreal/BP/Interface/BPI_DimensionObject.ActiveObject`
  (params (Material :type "MaterialInstance Object Reference"))
  (`PrimitiveComponent.SetCollisionEnabled` (`self.Plane`) "QueryAndPhysics"))

(event `/Game/ProjerUnreal/BP/Interface/BPI_DimensionObject.DisableObject`
  (`PrimitiveComponent.SetCollisionEnabled` (`self.Plane`) "NoCollision"))

(fn `GetArrow`
  (returns (Arrow :type "ArrowComponent Object Reference"))
  (return (`self.Arrow`)))

(fn `GetRightArrow`
  (returns (Arrow :type "ArrowComponent Object Reference"))
  (return (`self.ArrowRight`)))

(fn `UserConstructionScript`
  (`parent.UserConstructionScript`))