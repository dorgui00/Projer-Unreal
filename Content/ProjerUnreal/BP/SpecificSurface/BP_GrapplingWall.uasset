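; BP_GrapplingWall is a wall actor, named as a grappling surface, that can be switched on and off and re-skinned through events.
; SetMaterial swaps the first material slot on its Cube.
; DisableObject turns off Box collision at once, then hides Box and its children after a short delay.
; ActiveObject restores collision and visibility immediately.
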(event `/Game/ProjerUnreal/BP/Interface/BPI_DimensionObject.SetMaterial`
  (params (Mat :type "MaterialInstance Object Reference"))
  (`PrimitiveComponent.SetMaterial` (`self.Cube`) 0 Mat))

(event `/Game/ProjerUnreal/BP/Interface/BPI_DimensionObject.DisableObject`
  (`PrimitiveComponent.SetCollisionEnabled` (`self.Box`) "NoCollision")
  (`KismetSystemLibrary.Delay` 0.5)
  (`SceneComponent.SetVisibility` (`self.Box`) false true))

(event `/Game/ProjerUnreal/BP/Interface/BPI_DimensionObject.ActiveObject`
  (`PrimitiveComponent.SetCollisionEnabled` (`self.Box`) "QueryAndPhysics")
  (`SceneComponent.SetVisibility` (`self.Box`) true true))

(fn `UserConstructionScript`)