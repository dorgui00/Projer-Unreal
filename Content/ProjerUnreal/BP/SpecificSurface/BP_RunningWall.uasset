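; BP_RunningWall is a plane-based running wall surface that can exist in the Past dimension, the Futur dimension or both.
; SetMaterial swaps the plane's material to match the given dimension.
; ActiveObject turns on collision and shows the whole component hierarchy at once.
; DisableObject removes collision immediately but hides the hierarchy after a short delay, so the wall stays visible briefly after it stops blocking.
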(event `/Game/ProjerUnreal/BP/Interface/BPI_DimensionObject.SetMaterial`
  (params (Dimension :type "/Game/ProjerUnreal/Data/E_Dimensions Enum" :default "NewEnumerator0"))
  (switch `/Game/ProjerUnreal/Data/E_Dimensions` Dimension
    (:`NewEnumerator0`
      (`PrimitiveComponent.SetMaterial` (`self.Plane`) 0 (`self.PastMaterial`)))
    (:`NewEnumerator1`
      (`PrimitiveComponent.SetMaterial` (`self.Plane`) 0 (`self.FuturMaterial`)))
    (:`NewEnumerator2`
      (`PrimitiveComponent.SetMaterial` (`self.Plane`) 0 (`self.BothMaterial`)))))

(event `/Game/ProjerUnreal/BP/Interface/BPI_DimensionObject.DisableObject`
  (`PrimitiveComponent.SetCollisionEnabled` (`self.Plane`) "NoCollision")
  (`KismetSystemLibrary.Delay` 0.8)
  (`SceneComponent.SetVisibility` (`self.DefaultSceneRoot`) false true))

(event `/Game/ProjerUnreal/BP/Interface/BPI_DimensionObject.ActiveObject`
  (`PrimitiveComponent.SetCollisionEnabled` (`self.Plane`) "QueryAndPhysics")
  (`SceneComponent.SetVisibility` (`self.DefaultSceneRoot`) true true))

(fn `UserConstructionScript`)