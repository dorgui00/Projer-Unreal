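; BP_CheckPoint is a checkpoint actor that reports itself to the Game Instance when a character touches it.
; Both begin and end overlap on its CheckPoint component check that the other actor implements BPI_Character.
; On a match, either event passes the checkpoint to the Game Instance through SetNewCheckpointMessage, so leaving the volume registers it again.
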(event `self.CheckPoint.OnComponentBeginOverlap`
  (params (OverlappedComponent :type "PrimitiveComponent Object Reference") (OtherActor :type "Actor Object Reference") (OtherComp :type "PrimitiveComponent Object Reference") (OtherBodyIndex :type Integer) (bFromSweep :type Boolean) (SweepResult :type "HitResult Structure (by ref)"))
  (if (`KismetSystemLibrary.DoesImplementInterface` OtherActor "/Game/ProjerUnreal/BP/Interface/BPI_Character.BPI_Character_C")
    (message `/Game/ProjerUnreal/BP/Interface/BPI_GI.SetNewCheckpoint` (`GameplayStatics.GetGameInstance`) self)))

(event `self.CheckPoint.OnComponentEndOverlap`
  (params (OverlappedComponent :type "PrimitiveComponent Object Reference") (OtherActor :type "Actor Object Reference") (OtherComp :type "PrimitiveComponent Object Reference") (OtherBodyIndex :type Integer))
  (if (`KismetSystemLibrary.DoesImplementInterface` OtherActor "/Game/ProjerUnreal/BP/Interface/BPI_Character.BPI_Character_C")
    (message `/Game/ProjerUnreal/BP/Interface/BPI_GI.SetNewCheckpoint` (`GameplayStatics.GetGameInstance`) self)))

(fn `UserConstructionScript`)