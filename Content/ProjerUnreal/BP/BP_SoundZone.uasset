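; BP_SoundZone is an actor that plays a past or future sound depending on the current dimension.
; On BeginPlay it assigns both sounds and shared attenuation settings to two audio components, then binds an event to the game instance's dimension-swap dispatcher in GI_Main.
; Its Activet event reads the dimension from the game instance, stops one component and plays the other from the start.
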(event `self.ReceiveBeginPlay`
  (`AudioComponent.SetSound` (`self.SoudsFutur`) (`self.New SoundFutur`))
  (`AudioComponent.SetSound` (`self.SoudsPaser`) (`self.New SoundPasser`))
  (set `AudioComponent.AttenuationSettings` (`self.Attenuation Settings`) (`self.SoudsFutur`))
  (set `AudioComponent.AttenuationSettings` (`self.Attenuation Settings`) (`self.SoudsPaser`))
  (bind _asgi_main (cast `/Game/ProjerUnreal/BP/GI_Main` (`GameplayStatics.GetGameInstance`)))
  (add `/Game/ProjerUnreal/BP/GI_Main.ED_SwapDimension` _asgi_main (`|CreateDelegate` :!event `Activet`)))

(event `/Game/ProjerUnreal/BP/Interface/BPI_Song.Activet`
  (bind _dimension (message `/Game/ProjerUnreal/BP/Interface/BPI_GI.GetDimension` (`GameplayStatics.GetGameInstance`)))
  (if (`|EnumEquality` _dimension "NewEnumerator1")
    (`AudioComponent.Stop` (`self.SoudsPaser`))
    (`AudioComponent.Play` (`self.SoudsFutur`) 0.0)
    (else
      (`AudioComponent.Stop` (`self.SoudsFutur`))
      (`AudioComponent.Play` (`self.SoudsPaser`) 0.0))))

(fn `UserConstructionScript`)