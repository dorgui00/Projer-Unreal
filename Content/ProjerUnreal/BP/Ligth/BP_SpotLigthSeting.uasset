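; Spot light actor that changes its look between the past and future dimensions, with separate intensity, color and shadow casting for each.
; BeginPlay binds to the GI_Main game instance's dimension-swap dispatcher and applies the shared cone and source shape settings.
; LateNuis applies the look matching the game instance's current dimension, treating Both as Past.
; SWITCH uses a FlipFlop to alternate looks, starting with future, and reapplies the shape settings.
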(event `self.ReceiveBeginPlay`
  (bind _asgi_main (cast `/Game/ProjerUnreal/BP/System/GI_Main` (`GameplayStatics.GetGameInstance`)))
  (add `/Game/ProjerUnreal/BP/System/GI_Main.ED_SwapDimension` _asgi_main (`|CreateDelegate` :!event `LateNuis`))
  (`SpotLightComponent.SetInnerConeAngle` (`self.SpotLight`) (`self.New Inner Cone Angle`))
  (`SpotLightComponent.SetOuterConeAngle` (`self.SpotLight`) (`self.New Outer Cone Angle`))
  (`PointLightComponent.SetSourceRadius` (`self.SpotLight`) (`self.New Source Radius`))
  (`PointLightComponent.SetSoftSourceRadius` (`self.SpotLight`) (`self.New Soft Source Radius`))
  (`PointLightComponent.SetSourceLength` (`self.SpotLight`) (`self.New Source Length`)))

(event `LateNuis`
  (bind _dimension (message `/Game/ProjerUnreal/BP/Interface/BPI_GI.GetDimension` (`GameplayStatics.GetGameInstance`)))
  (switch `/Game/ProjerUnreal/Data/E_Dimensions` _dimension
    (:`NewEnumerator0`
      (`LightComponent.SetIntensity` (`self.SpotLight`) (`self.PASSER Intensity`) :!label _label)
      (`LightComponent.SetLightColor` (`self.SpotLight`) (`self.PASSER Light Color`) true)
      (`LightComponentBase.SetCastShadows` (`self.SpotLight`) (`self.PASSER Cast Shadows`)))
    (:`NewEnumerator1`
      (`LightComponent.SetIntensity` (`self.SpotLight`) (`self.FUTURRE Intensity`))
      (`LightComponent.SetLightColor` (`self.SpotLight`) (`self.FUTURE Light Color`) true)
      (`LightComponentBase.SetCastShadows` (`self.SpotLight`) (`self.FUTURRE Cast Shadows`)))
    (:`NewEnumerator2`
      (goto _label))))

(event `SWITCH`
  (`/Engine/EditorBlueprintResources/StandardMacros.FlipFlop`
    (:`A`
      (`LightComponent.SetIntensity` (`self.SpotLight`) (`self.FUTURRE Intensity`))
      (`LightComponent.SetLightColor` (`self.SpotLight`) (`self.FUTURE Light Color`) true)
      (`LightComponentBase.SetCastShadows` (`self.SpotLight`) (`self.FUTURRE Cast Shadows`))
      (`SpotLightComponent.SetInnerConeAngle` (`self.SpotLight`) (`self.New Inner Cone Angle`))
      (`SpotLightComponent.SetOuterConeAngle` (`self.SpotLight`) (`self.New Outer Cone Angle`))
      (`PointLightComponent.SetSourceRadius` (`self.SpotLight`) (`self.New Source Radius`))
      (`PointLightComponent.SetSoftSourceRadius` (`self.SpotLight`) (`self.New Soft Source Radius`))
      (`PointLightComponent.SetSourceLength` (`self.SpotLight`) (`self.New Source Length`)))
    (:`B`
      (`LightComponent.SetIntensity` (`self.SpotLight`) (`self.PASSER Intensity`))
      (`LightComponent.SetLightColor` (`self.SpotLight`) (`self.PASSER Light Color`) true)
      (`LightComponentBase.SetCastShadows` (`self.SpotLight`) (`self.PASSER Cast Shadows`))
      (`SpotLightComponent.SetInnerConeAngle` (`self.SpotLight`) (`self.New Inner Cone Angle`))
      (`SpotLightComponent.SetOuterConeAngle` (`self.SpotLight`) (`self.New Outer Cone Angle`))
      (`PointLightComponent.SetSourceRadius` (`self.SpotLight`) (`self.New Source Radius`))
      (`PointLightComponent.SetSoftSourceRadius` (`self.SpotLight`) (`self.New Soft Source Radius`))
      (`PointLightComponent.SetSourceLength` (`self.SpotLight`) (`self.New Source Length`)))))

(fn `UserConstructionScript`)