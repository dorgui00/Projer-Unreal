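; Light-setting Blueprint that toggles SkyLight shadow casting according to the game's past or future time dimension.
; On BeginPlay it binds an event to GI_Main's swap-dimension dispatcher.
; LateNuis reads the current dimension from the game instance and applies the Past or Futur shadow setting, treating Both as Past.
; Separate PASSER and FUTURRE events apply each setting directly.
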(event `self.ReceiveBeginPlay`
  (bind _asgi_main (cast `/Game/ProjerUnreal/BP/GI_Main` (`GameplayStatics.GetGameInstance`)))
  (add `/Game/ProjerUnreal/BP/GI_Main.ED_SwapDimension` _asgi_main (`|CreateDelegate` :!event `LateNuis`)))

(event `LateNuis`
  (bind _dimension (message `/Game/ProjerUnreal/BP/Interface/BPI_GI.GetDimension` (`GameplayStatics.GetGameInstance`)))
  (switch `/Game/ProjerUnreal/Data/E_Dimensions` _dimension
    (:`NewEnumerator0`
      (`LightComponentBase.SetCastShadows` (`self.SkyLight`) (`self.PASSER Cast Shadows`) :!label _label))
    (:`NewEnumerator1`
      (`LightComponentBase.SetCastShadows` (`self.SkyLight`) (`self.FUTURRE Cast Shadows`)))
    (:`NewEnumerator2`
      (goto _label))))

(event `FUTURRE`
  (`LightComponentBase.SetCastShadows` (`self.SkyLight`) (`self.FUTURRE Cast Shadows`)))

(event `PASSER`
  (`LightComponentBase.SetCastShadows` (`self.SkyLight`) (`self.PASSER Cast Shadows`)))

(fn `UserConstructionScript`)