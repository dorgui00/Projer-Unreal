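; Rect light actor that changes its look between the Past and Future dimensions.
; On BeginPlay it binds to GI_Main's dimension-swap dispatcher and applies radius, source size and barn door settings from variables.
; LateNuis reads the game instance's dimension and sets intensity and color, treating Both as Past.
; Separate PASSER and FUTURRE events apply each full preset, including shadow casting.
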(event `self.ReceiveBeginPlay`
  (bind _asgi_main (cast `/Game/ProjerUnreal/BP/System/GI_Main` (`GameplayStatics.GetGameInstance`)))
  (add `/Game/ProjerUnreal/BP/System/GI_Main.ED_SwapDimension` _asgi_main (`|CreateDelegate` :!event `LateNuis`))
  (`LocalLightComponent.SetAttenuationRadius` (`self.RectLight`) (`self.New Radius`))
  (`RectLightComponent.SetSourceWidth` (`self.RectLight`) (`self.NewSourceWidth`))
  (`RectLightComponent.SetSourceHeight` (`self.RectLight`) (`self.NewSourceHeight`))
  (`RectLightComponent.SetBarnDoorAngle` (`self.RectLight`) (`self.NewBarnDoorAngle`))
  (`RectLightComponent.SetBarnDoorLength` (`self.RectLight`) (`self.NewBaenLength`)))

(event `LateNuis`
  (bind _dimension (message `/Game/ProjerUnreal/BP/Interface/BPI_GI.GetDimension` (`GameplayStatics.GetGameInstance`)))
  (switch `/Game/ProjerUnreal/Data/E_Dimensions` _dimension
    (:`NewEnumerator0`
      (`LightComponent.SetIntensity` (`self.RectLight`) (`self.PASSER Intensity`) :!label _label)
      (`LightComponent.SetLightColor` (`self.RectLight`) (`self.PASSER Light Color`) true))
    (:`NewEnumerator1`
      (`LightComponent.SetIntensity` (`self.RectLight`) (`self.FUTURE Intensity`))
      (`LightComponent.SetLightColor` (`self.RectLight`) (`self.FUTURE Light Color`) true))
    (:`NewEnumerator2`
      (goto _label))))

(event `FUTURRE`
  (`LightComponent.SetIntensity` (`self.RectLight`) (`self.FUTURE Intensity`))
  (`LightComponent.SetLightColor` (`self.RectLight`) (`self.FUTURE Light Color`) true)
  (`LightComponentBase.SetCastShadows` (`self.RectLight`) (`self.FUTURE Cast Shadows`))
  (`LocalLightComponent.SetAttenuationRadius` (`self.RectLight`) (`self.New Radius`))
  (`RectLightComponent.SetSourceWidth` (`self.RectLight`) (`self.NewSourceWidth`))
  (`RectLightComponent.SetSourceHeight` (`self.RectLight`) (`self.NewSourceHeight`))
  (`RectLightComponent.SetBarnDoorAngle` (`self.RectLight`) (`self.NewBarnDoorAngle`))
  (`RectLightComponent.SetBarnDoorLength` (`self.RectLight`) (`self.NewBaenLength`)))

(event `PASSER`
  (`LightComponent.SetIntensity` (`self.RectLight`) (`self.PASSER Intensity`))
  (`LightComponent.SetLightColor` (`self.RectLight`) (`self.PASSER Light Color`) true)
  (`LightComponentBase.SetCastShadows` (`self.RectLight`) (`self.PASSER Cast Shadows`))
  (`LocalLightComponent.SetAttenuationRadius` (`self.RectLight`) (`self.New Radius`))
  (`RectLightComponent.SetSourceWidth` (`self.RectLight`) (`self.NewSourceWidth`))
  (`RectLightComponent.SetSourceHeight` (`self.RectLight`) (`self.NewSourceHeight`))
  (`RectLightComponent.SetBarnDoorAngle` (`self.RectLight`) (`self.NewBarnDoorAngle`))
  (`RectLightComponent.SetBarnDoorLength` (`self.RectLight`) (`self.NewBaenLength`)))

(fn `UserConstructionScript`)