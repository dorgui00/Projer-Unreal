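; Point light actor whose intensity, color and shadow casting change with the game's Past or Futur dimension.
; On BeginPlay it binds to GI_Main's dimension-swap dispatcher, runs SwapLight and sets the source shape.
; SwapLight reads the dimension from the game instance and applies the matching variable set, with Both using Past values.
; Separate FUTUR and PASSER events apply either look directly, including source shape.
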(event `self.ReceiveBeginPlay`
  (bind _asgi_main (cast `/Game/ProjerUnreal/BP/GI_Main` (`GameplayStatics.GetGameInstance`)))
  (add `/Game/ProjerUnreal/BP/GI_Main.ED_SwapDimension` _asgi_main (`|CreateDelegate` :!event `SwapLight`))
  (`self.SwapLight`)
  (`PointLightComponent.SetSourceRadius` (`self.PointLight`) (`self.New Source Radius`))
  (`PointLightComponent.SetSoftSourceRadius` (`self.PointLight`) (`self.New Soft Source Radius`))
  (`PointLightComponent.SetSourceLength` (`self.PointLight`) (`self.New Source Length`)))

(event `SwapLight`
  (bind _dimension (message `/Game/ProjerUnreal/BP/Interface/BPI_GI.GetDimension` (`GameplayStatics.GetGameInstance`)))
  (switch `/Game/ProjerUnreal/Data/E_Dimensions` _dimension
    (:`NewEnumerator0`
      (`LightComponent.SetIntensity` (`self.PointLight`) (`self.PASSER Intensity`) :!label _label)
      (`LightComponent.SetLightColor` (`self.PointLight`) (`self.PASSER Light Color`) true)
      (`LightComponentBase.SetCastShadows` (`self.PointLight`) (`self.PASSER Cast Shadows`)))
    (:`NewEnumerator1`
      (`LightComponent.SetIntensity` (`self.PointLight`) (`self.FUTURRE Intensity`))
      (`LightComponent.SetLightColor` (`self.PointLight`) (`self.FUTURE Light Color`) true)
      (`LightComponentBase.SetCastShadows` (`self.PointLight`) (`self.FUTURRE Cast Shadows`)))
    (:`NewEnumerator2`
      (goto _label))))

(event `FUTUR`
  (`LightComponent.SetIntensity` (`self.PointLight`) (`self.FUTURRE Intensity`))
  (`LightComponent.SetLightColor` (`self.PointLight`) (`self.FUTURE Light Color`) true)
  (`LightComponentBase.SetCastShadows` (`self.PointLight`) (`self.FUTURRE Cast Shadows`))
  (`PointLightComponent.SetSourceRadius` (`self.PointLight`) (`self.New Source Radius`))
  (`PointLightComponent.SetSoftSourceRadius` (`self.PointLight`) (`self.New Soft Source Radius`))
  (`PointLightComponent.SetSourceLength` (`self.PointLight`) (`self.New Source Length`)))

(event `PASSER`
  (`LightComponent.SetIntensity` (`self.PointLight`) (`self.PASSER Intensity`))
  (`LightComponent.SetLightColor` (`self.PointLight`) (`self.PASSER Light Color`) true)
  (`LightComponentBase.SetCastShadows` (`self.PointLight`) (`self.PASSER Cast Shadows`))
  (`PointLightComponent.SetSourceRadius` (`self.PointLight`) (`self.New Source Radius`))
  (`PointLightComponent.SetSoftSourceRadius` (`self.PointLight`) (`self.New Soft Source Radius`))
  (`PointLightComponent.SetSourceLength` (`self.PointLight`) (`self.New Source Length`)))

(fn `UserConstructionScript`)