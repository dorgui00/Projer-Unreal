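; Actor Blueprint that drives the visual transition of a past/present dimension swap through the DimensionMaterialParameter collection.
; On BeginPlay it binds to the GI_Main swap-dimension dispatcher.
; Its update event stores the player capsule position, then plays a timeline using the swap duration as play rate to ramp Scalar and flag IsMoving.
; When finished, it flips IsPast and resets both transition parameters.
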(event `self.ReceiveBeginPlay`
  (bind _asgi_main (cast `/Game/ProjerUnreal/BP/GI_Main` (`GameplayStatics.GetGameInstance`)))
  (bind _output_get (set `self.GameInstance` _asgi_main))
  (add `/Game/ProjerUnreal/BP/GI_Main.ED_SwapDimension` _output_get (`|CreateDelegate` :!event `CE_UpdateMaterial`)))

(event `CE_UpdateMaterial`
  (bind (_returnvalue_x _returnvalue_y _returnvalue_z) (`KismetMathLibrary.BreakVector` (`SceneComponent.K2_GetComponentLocation` (`Character.CapsuleComponent` (`GameplayStatics.GetPlayerCharacter` 0)))))
  (`KismetMaterialLibrary.SetVectorParameterValue` "/Game/ProjerUnreal/Materials/DimensionMaterialParameter.DimensionMaterialParameter" "PlayerPos" (make `LinearColor` _returnvalue_x _returnvalue_y _returnvalue_z))
  (bind _duration (`/Game/ProjerUnreal/BP/Interface/BPI_GI.GetSwapDuration` (`self.GameInstance`)))
  (`TimelineComponent.SetPlayRate` (`self.Timeline`) _duration)
  (bind (_direction _interfloat) (`Timeline|Timeline` :!via `PlayFromStart`)
    (:`Update`
      (`KismetMaterialLibrary.SetScalarParameterValue` "/Game/ProjerUnreal/Materials/DimensionMaterialParameter.DimensionMaterialParameter" "Scalar" (`KismetMathLibrary.Lerp` 0.0 1.0 _interfloat))
      (`KismetMaterialLibrary.SetScalarParameterValue` "/Game/ProjerUnreal/Materials/DimensionMaterialParameter.DimensionMaterialParameter" "IsMoving" 1.0))
    (:`Finished`
      (bind _returnvalue (`KismetMaterialLibrary.GetScalarParameterValue` "/Game/ProjerUnreal/Materials/DimensionMaterialParameter.DimensionMaterialParameter" "IsPast"))
      (`KismetMaterialLibrary.SetScalarParameterValue` "/Game/ProjerUnreal/Materials/DimensionMaterialParameter.DimensionMaterialParameter" "IsPast" (- 1.0 _returnvalue))
      (`KismetMaterialLibrary.SetScalarParameterValue` "/Game/ProjerUnreal/Materials/DimensionMaterialParameter.DimensionMaterialParameter" "IsMoving")
      (`KismetMaterialLibrary.SetScalarParameterValue` "/Game/ProjerUnreal/Materials/DimensionMaterialParameter.DimensionMaterialParameter" "Scalar"))))

(fn `UserConstructionScript`)