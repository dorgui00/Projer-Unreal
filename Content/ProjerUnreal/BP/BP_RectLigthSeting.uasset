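; BP_RectLigthSeting is a configurable rect light whose brightness differs between the game's future and past dimensions.
; On BeginPlay it binds to GI_Main's dimension-swap event dispatcher and applies its variables for color, attenuation radius, source size and barn doors.
; The LateNuis event reads the current dimension from the game instance and sets either the future or the past intensity.
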(event `self.ReceiveBeginPlay`
  (bind _asgi_main (cast `/Game/ProjerUnreal/BP/System/GI_Main` (`GameplayStatics.GetGameInstance`)))
  (add `/Game/ProjerUnreal/BP/System/GI_Main.ED_SwapDimension` _asgi_main (`|CreateDelegate` :!event `LateNuis`))
  (`LightComponent.SetLightColor` (`self.RectLight`) (`self.New Light Color`) true)
  (`LocalLightComponent.SetAttenuationRadius` (`self.RectLight`) (`self.New Radius`))
  (`RectLightComponent.SetSourceWidth` (`self.RectLight`) (`self.NewSourceWidth`))
  (`RectLightComponent.SetSourceHeight` (`self.RectLight`) (`self.NewSourceHeight`))
  (`RectLightComponent.SetBarnDoorAngle` (`self.RectLight`) (`self.NewBarnDoorAngle`))
  (`RectLightComponent.SetBarnDoorLength` (`self.RectLight`) (`self.NewBaenLength`)))

(event `LateNuis`
  (bind _dimension (message `/Game/ProjerUnreal/BP/Interface/BPI_GI.GetDimension` (`GameplayStatics.GetGameInstance`)))
  (if (`|EnumEquality` _dimension "NewEnumerator1")
    (`LightComponent.SetIntensity` (`self.RectLight`) (`self.New IntensityFutur`))
    (else
      (`LightComponent.SetIntensity` (`self.RectLight`) (`self.New IntensityPasser`)))))

(fn `UserConstructionScript`)