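; Character component that fires a grappling hook along the first-person camera and pulls the player toward grappling walls.
; CE_Grappling line traces up to MaxRange, spawns a BP_Hook with the character's cable attached, and moves it to the hit or full range.
; A BP_GrapplingWall hit lowers gravity and launches the character toward it, then after Duration restores gravity and damps velocity.
; IsGrappling blocks re-firing until the hook is destroyed.
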(event `CE_Grappling`
  (params (Character :type "/Game/ProjerUnreal/BP/Character/BP_Character Object Reference"))
  (bind _charactermovement (`Character.CharacterMovement` (`self.Character`)))
  (set `self.Character` Character)
  (set `self.InitialPosition` (`Actor.K2_GetActorLocation` Character))
  (set `self.CableRef` (`/Game/ProjerUnreal/BP/Character/BP_Character.Cable` Character))
  (if (not (`self.isGrappling`))
    (set `self.isGrappling` true)
    (bind (_outhit _returnvalue) (`KismetSystemLibrary.LineTraceSingle` (`Actor.K2_GetActorLocation` (`self.Character`)) (+ (`self.InitialPosition`) (* (`SceneComponent.GetForwardVector` (`/Game/ProjerUnreal/BP/Character/BP_Character.FirstPersonCamera` (`self.Character`))) (`self.Max Range`))) "TraceTypeQuery4"))
    (if _returnvalue
      (bind (_bblockinghit _binitialoverlap _time _distance _location _impactpoint _normal _impactnormal _physmat _hitactor) (`GameplayStatics.BreakHitResult` _outhit))
      (set `self.ImpactPoint` _impactpoint)
      (if (< (`KismetMathLibrary.Vector_Distance` (`self.ImpactPoint`) (`self.InitialPosition`)) (`self.Max Range`))
        (bind _returnvalue_2 (`|SpawnActorFromClass` "/Game/ProjerUnreal/BP/Character/BP_Hook.BP_Hook_C" (`Actor.GetTransform` (`self.Character`)) "Undefined" "MultiplyWithRoot" null null))
        (`CableComponent.SetAttachEndToComponent` (`self.CableRef`) (`Actor.RootComponent` _returnvalue_2) "None")
        (`KismetSystemLibrary.MoveComponentTo` (`Actor.RootComponent` _returnvalue_2) (`self.ImpactPoint`))
        (cast `/Game/ProjerUnreal/BP/SpecificSurface/BP_GrapplingWall` _hitactor
          (:`then`
            (set `CharacterMovementComponent.GravityScale` 1.0 (`Character.CharacterMovement` (`self.Character`)))
            (`Character.LaunchCharacter` (`self.Character`) (* (`KismetMathLibrary.Normal` (- (`self.ImpactPoint`) (`self.InitialPosition`))) 3000.0) true true)
            (`KismetSystemLibrary.Delay` (`self.Duration`))
            (set `CharacterMovementComponent.GravityScale` 2.0 _charactermovement)
            (set `MovementComponent.Velocity` (/ (`MovementComponent.Velocity` _charactermovement) (`self.VelocityReduce`)) _charactermovement)
            (set `self.isGrappling` false)
            (`Actor.K2_DestroyActor` _returnvalue_2))
          (:`CastFailed`
            (set `self.isGrappling` false)
            (`Actor.K2_DestroyActor` _returnvalue_2)))
        (else
          (bind _returnvalue_3 (`|SpawnActorFromClass` "/Game/ProjerUnreal/BP/Character/BP_Hook.BP_Hook_C" (`Actor.GetTransform` (`self.Character`)) "Undefined" "MultiplyWithRoot" null null :!label _label))
          (`CableComponent.SetAttachEndToComponent` (`self.CableRef`) (`Actor.RootComponent` _returnvalue_3) "None")
          (`KismetSystemLibrary.MoveComponentTo` (`Actor.RootComponent` _returnvalue_3) (+ (`Actor.K2_GetActorLocation` (`self.Character`)) (* (`SceneComponent.GetForwardVector` (`/Game/ProjerUnreal/BP/Character/BP_Character.FirstPersonCamera` (`self.Character`))) (`self.Max Range`))))
          (set `CharacterMovementComponent.GravityScale` 2.0 (`Character.CharacterMovement` (`self.Character`)))
          (`Actor.K2_DestroyActor` _returnvalue_3)
          (set `self.isGrappling` false)))
      (else
        (goto _label)))))