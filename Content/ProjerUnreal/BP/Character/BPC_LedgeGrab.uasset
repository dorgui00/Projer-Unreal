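; Character component that detects climbable ledges in front of a given character, setting CanLedgeClimb and a PositionLedge target above the ledge.
; CE_LedgeGrab traces forward for a wall, then downward from above to find the ledge top.
; VerifBehind rejects ledges with obstructions along or behind the approach, while an upward trace and Verif's four offset traces check clearance above.
; All checks use Visibility line traces, and failed checks disallow climbing.
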(event `CE_LedgeGrab`
  (params (Perso :type "Actor Object Reference"))
  (bind _perso (`self.Perso`))
  (bind _perso_2 (`self.Perso`))
  (bind (_returnvalue_x _returnvalue_y _returnvalue_z) (`KismetMathLibrary.BreakVector` (`Actor.K2_GetActorLocation` _perso_2)))
  (bind _returnvalue (`Actor.GetActorUpVector` _perso))
  (bind _returnvalue_2 (+ (`Actor.K2_GetActorLocation` _perso) (+ (* (`Actor.GetActorForwardVector` _perso) 75.0) (* _returnvalue 120.0))))
  (set `self.Perso` Perso)
  (bind _outhit (`KismetSystemLibrary.LineTraceSingle` (`KismetMathLibrary.MakeVector` _returnvalue_x _returnvalue_y _returnvalue_z) (+ (`KismetMathLibrary.MakeVector` _returnvalue_x _returnvalue_y (+ _returnvalue_z 50.0)) (* (`Actor.GetActorForwardVector` _perso_2) 75.0)) "TraceTypeQuery1"))
  (bind _bblockinghit (`GameplayStatics.BreakHitResult` _outhit))
  (if _bblockinghit
    (bind (_outhit_2 _returnvalue_3) (`KismetSystemLibrary.LineTraceSingle` _returnvalue_2 (+ _returnvalue_2 (* _returnvalue -150.0)) "TraceTypeQuery1"))
    (if _returnvalue_3
      (bind (_bblockinghit_2 _binitialoverlap _time _distance _location _impactpoint) (`GameplayStatics.BreakHitResult` _outhit_2))
      (bind _touch (`self.VerifBehind` (+ _impactpoint (* (`Actor.GetActorForwardVector` (`self.Perso`)) 30.0))))
      (if _touch
        (set `self.CanLedgeClimb` false)
        (set `self.PositionLedge` (0.0 0.0 0.0))
        (else
          (bind _returnvalue_4 (+ _impactpoint (0.0 0.0 20.0)))
          (set `self.Start` _returnvalue_4)
          (bind _returnvalue_5 (+ _impactpoint (0.0 0.0 100.0)))
          (set `self.End` _returnvalue_5)
          (bind (_outhit_3 _returnvalue_6) (`KismetSystemLibrary.LineTraceSingle` _returnvalue_4 _returnvalue_5 "TraceTypeQuery1"))
          (bind _touch_2 (`self.Verif` (`self.Start`) (`self.End`)))
          (if (or _touch_2 _returnvalue_6)
            (set `self.CanLedgeClimb` false)
            (set `self.PositionLedge` (0.0 0.0 0.0))
            (else
              (set `self.CanLedgeClimb` (not _returnvalue_6))
              (set `self.PositionLedge` _returnvalue_5))))))
    (else
      (set `self.CanLedgeClimb` _bblockinghit)
      (set `self.PositionLedge` (0.0 0.0 0.0)))))

(fn `Verif`
  (params (Start :type "Vector Structure") (End :type "Vector Structure"))
  (returns (Touch :type Boolean))
  (bind (_outhit _returnvalue) (`KismetSystemLibrary.LineTraceSingle` (+ Start (20.0 0.0 0.0)) (+ End (40.0 0.0 30.0)) "TraceTypeQuery1"))
  (bind (_outhit_2 _returnvalue_2) (`KismetSystemLibrary.LineTraceSingle` (- Start (20.0 0.0 0.0)) (- End (40.0 0.0 30.0)) "TraceTypeQuery1"))
  (bind (_outhit_3 _returnvalue_3) (`KismetSystemLibrary.LineTraceSingle` (+ Start (0.0 20.0 0.0)) (+ End (0.0 40.0 30.0)) "TraceTypeQuery1"))
  (bind (_outhit_4 _returnvalue_4) (`KismetSystemLibrary.LineTraceSingle` (- Start (0.0 20.0 0.0)) (- End (0.0 40.0 30.0)) "TraceTypeQuery1"))
  (return (or (or _returnvalue_4 _returnvalue_2) (or _returnvalue_3 _returnvalue))))

(fn `VerifBehind`
  (params (Start :type "Vector Structure"))
  (returns (Touch :type Boolean))
  (bind _returnvalue (+ Start (0.0 0.0 30.0)))
  (bind _returnvalue_2 (- Start (* (`Actor.GetActorForwardVector` (`self.Perso`)) 300.0)))
  (bind _returnvalue_3 (+ (- Start (* (`Actor.GetActorForwardVector` (`self.Perso`)) 100.0)) (0.0 0.0 30.0)))
  (bind (_outhit _returnvalue_4) (`KismetSystemLibrary.LineTraceSingle` _returnvalue _returnvalue_3 "TraceTypeQuery1"))
  (bind (_outhit_2 _returnvalue_5) (`KismetSystemLibrary.LineTraceSingle` _returnvalue_3 _returnvalue "TraceTypeQuery1"))
  (bind (_outhit_3 _returnvalue_6) (`KismetSystemLibrary.LineTraceSingle` (- _returnvalue_2 (0.0 0.0 200.0)) (+ _returnvalue_2 (0.0 0.0 100.0)) "TraceTypeQuery1"))
  (return (or (or _returnvalue_4 _returnvalue_5) _returnvalue_6)))