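; BP_MenuPawn is the menu pawn, handling dimension swap and scroll input and starting menu audio and save loading.
; On controller change it resets Enhanced Input to IMC_Default and registers that context with user settings if needed.
; Swap calls the BPCSwapDimension component behind a short delay-based cooldown, while scroll actions fire event dispatchers.
; BeginPlay sets the main sound mix and calls LoadSaveMessage on the game instance.
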(event `self.ReceiveControllerChanged`
  (params (OldController :type "Controller Object Reference") (NewController :type "Controller Object Reference"))
  (bind _asplayer_controller (cast `PlayerController` NewController))
  (bind _returnvalue (pcsubsystem `EnhancedInputLocalPlayerSubsystem` _asplayer_controller))
  (`EnhancedInputSubsystemInterface.ClearAllMappings` _returnvalue)
  (`EnhancedInputSubsystemInterface.AddMappingContext` _returnvalue "/Game/FirstPerson/Input/IMC_Default.IMC_Default" 0 (struct))
  (bind _returnvalue_2 (`EnhancedInputSubsystemInterface.GetUserSettings` _returnvalue))
  (if (not (`EnhancedInputUserSettings.IsMappingContextRegistered` _returnvalue_2 "/Game/FirstPerson/Input/IMC_Default.IMC_Default"))
    (`EnhancedInputUserSettings.RegisterInputMappingContext` _returnvalue_2 "/Game/FirstPerson/Input/IMC_Default.IMC_Default")))

(event `EnhancedInput|/Game/FirstPerson/Input/Actions/IA_Swap`
  (params (ActionValue :type Boolean) (ElapsedSeconds :type "Float (double-precision)") (TriggeredSeconds :type "Float (double-precision)") (InputAction :type "InputAction Object Reference" :default "/Game/FirstPerson/Input/Actions/IA_Swap.IA_Swap"))
  (:`Started`
    (if (`self.Can Swap`)
      (set `self.Can Swap` false)
      (`/Game/ProjerUnreal/BP/Character/BPC_SwapDimension.CE_ChangeDimension` (`self.BPC_SwapDimension`))
      (`KismetSystemLibrary.Delay` 0.5)
      (set `self.Can Swap` true))))

(event `self.ReceiveBeginPlay`
  (`GameplayStatics.SetBaseSoundMix` "/Game/ProjerUnreal/BP/System/Sound/SM_Main.SM_Main")
  (message `/Game/ProjerUnreal/BP/Interface/BPI_GI.LoadSave` (`GameplayStatics.GetGameInstance`)))

(event `EnhancedInput|/Game/ProjerUnreal/Input/Action/IA_ScrollDown`
  (params (ActionValue :type "Float (double-precision)") (ElapsedSeconds :type "Float (double-precision)") (TriggeredSeconds :type "Float (double-precision)") (InputAction :type "InputAction Object Reference" :default "/Game/ProjerUnreal/Input/Action/IA_ScrollDown.IA_ScrollDown"))
  (:`Triggered`
    (`self.ED_ScrollDown`)))

(event `EnhancedInput|/Game/ProjerUnreal/Input/Action/IA_ScrollUp`
  (params (ActionValue :type "Float (double-precision)") (ElapsedSeconds :type "Float (double-precision)") (TriggeredSeconds :type "Float (double-precision)") (InputAction :type "InputAction Object Reference" :default "/Game/ProjerUnreal/Input/Action/IA_ScrollUp.IA_ScrollUp"))
  (:`Triggered`
    (`self.ED_ScrollUp`)))

(fn `UserConstructionScript`)