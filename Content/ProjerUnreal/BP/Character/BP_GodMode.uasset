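; BP_GodMode is a free-flying pawn with mouse-look style control and three-axis movement.
; On BeginPlay it adds the IMC_GodMode Enhanced Input mapping context to the first player controller.
; Look input drives controller yaw and pitch, while move input pushes along the actor's forward, right and up vectors.
; Each sprint press flip-flops the FloatingPawnMovement max speed between fast and slower values, so sprint is a toggle rather than a hold.
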(event `self.ReceiveBeginPlay`
  (`EnhancedInputSubsystemInterface.AddMappingContext` (pcsubsystem `EnhancedInputLocalPlayerSubsystem` (`GameplayStatics.GetPlayerController` 0)) "/Game/ProjerUnreal/Input/IMC_GodMode.IMC_GodMode" 0 (struct)))

(event `EnhancedInput|/Game/FirstPerson/Input/Actions/IA_Look`
  (params (ActionValue :type "Vector2D Structure") (ElapsedSeconds :type "Float (double-precision)") (TriggeredSeconds :type "Float (double-precision)") (InputAction :type "InputAction Object Reference" :default "/Game/FirstPerson/Input/Actions/IA_Look.IA_Look"))
  (bind (_x _y) (`KismetMathLibrary.BreakVector2D` ActionValue))
  ; Camera
  (:`Triggered`
    (`self.AddControllerYawInput` _x)
    (`self.AddControllerPitchInput` _y)))

(event `EnhancedInput|/Game/ProjerUnreal/Input/Action/IA_MoveGod`
  (params (ActionValue :type "Vector Structure") (ElapsedSeconds :type "Float (double-precision)") (TriggeredSeconds :type "Float (double-precision)") (InputAction :type "InputAction Object Reference" :default "/Game/ProjerUnreal/Input/Action/IA_MoveGod.IA_MoveGod"))
  ; Movement
  (:`Triggered`
    (`self.AddMovementInput` (`self.GetActorForwardVector`) (.y ActionValue))
    (`self.AddMovementInput` (`self.GetActorRightVector`) (.x ActionValue))
    (`self.AddMovementInput` (`self.GetActorUpVector`) (.z ActionValue))))

(event `EnhancedInput|/Game/ProjerUnreal/Input/Action/IA_Sprint`
  (params (ActionValue :type Boolean) (ElapsedSeconds :type "Float (double-precision)") (TriggeredSeconds :type "Float (double-precision)") (InputAction :type "InputAction Object Reference" :default "/Game/ProjerUnreal/Input/Action/IA_Sprint.IA_Sprint"))
  (:`Started`
    (`/Engine/EditorBlueprintResources/StandardMacros.FlipFlop`
      (:`A`
        (set `FloatingPawnMovement.MaxSpeed` 3000.0 (`self.FloatingPawnMovement`)))
      (:`B`
        (set `FloatingPawnMovement.MaxSpeed` 2000.0 (`self.FloatingPawnMovement`))))))

(fn `UserConstructionScript`)