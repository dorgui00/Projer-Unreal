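; BPC_Dash is a Blueprint component that gives a character a dash along the first-person camera's facing.
; Its CE_Dash event launches the passed character horizontally by the camera forward vector scaled by Distance, overriding XY velocity.
; An IsDashing flag blocks re-entry until Duration elapses, then the movement velocity is divided by DecelerationForce to brake the dash.
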(event `CE_Dash`
  (params (Character :type "/Game/ProjerUnreal/BP/Character/BP_Character Object Reference"))
  (set `self.Character` Character)
  (if (not (`self.isDashing`))
    (set `self.isDashing` true)
    (`Character.LaunchCharacter` (`self.Character`) (`KismetMathLibrary.MakeVector` (.x (* (`SceneComponent.GetForwardVector` (`/Game/ProjerUnreal/BP/Character/BP_Character.FirstPersonCamera` (`self.Character`))) (`self.Distance`))) (.y (* (`SceneComponent.GetForwardVector` (`/Game/ProjerUnreal/BP/Character/BP_Character.FirstPersonCamera` (`self.Character`))) (`self.Distance`)))) true false)
    (`KismetSystemLibrary.Delay` (`self.Duration`))
    (set `self.isDashing` false)
    (set `MovementComponent.Velocity` (/ (`MovementComponent.Velocity` (`Character.CharacterMovement` (`self.Character`))) (`self.DecelerationForce`)) (`Character.CharacterMovement` (`self.Character`)))))