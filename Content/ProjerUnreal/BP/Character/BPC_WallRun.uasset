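; Wall-run component that switches a character's movement in and out of a wall-running state.
; CE_StickToWall caches walk speed, lowers gravity, suppresses jump velocity and sets a vertical plane-constraint normal.
; If KeepJumpVelocityOnStick is set, it also zeroes vertical velocity and applies the wall-run speed.
; CE_UnstickToWall restores the cached speed, clears the constraint normal and resets gravity and jump to hardcoded values.
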(event `CE_StickToWall`
  (params (Character :type "/Game/ProjerUnreal/BP/Character/BP_Character Object Reference") (Wall :type "Actor Object Reference"))
  (bind _charactermovement (`Character.CharacterMovement` Character))
  (bind _character_movement (`self.Character Movement`))
  (bind (_velocity_x _velocity_y) (`KismetMathLibrary.BreakVector` (`MovementComponent.Velocity` _character_movement)))
  (if (`self.Debug`)
    (`KismetSystemLibrary.PrintString` "Stick to wall"))
  (set `self.Character Movement` _charactermovement)
  (set `self.InitialMaxSpeed` (`CharacterMovementComponent.MaxWalkSpeed` _charactermovement))
  (set `CharacterMovementComponent.bMaintainHorizontalGroundVelocity` true _charactermovement)
  (set `self.Wall` Wall)
  (set `self.IsWallRunning` true)
  (set `CharacterMovementComponent.JumpZVelocity` -1.0 _charactermovement)
  (set `CharacterMovementComponent.GravityScale` 0.1 (`self.Character Movement`))
  (`MovementComponent.SetPlaneConstraintNormal` _character_movement (0.0 0.0 1.0))
  (if (`self.KeepJumpVelocityOnStick`)
    (set `MovementComponent.Velocity` (`KismetMathLibrary.MakeVector` _velocity_x _velocity_y) _character_movement)
    (set `CharacterMovementComponent.MaxWalkSpeed` (`self.MaxSpeedWallRun`) _character_movement)))

(event `CE_UnstickToWall`
  (params (Character :type "/Game/ProjerUnreal/BP/Character/BP_Character Object Reference") (Wall :type "Actor Object Reference"))
  (bind _character_movement (`self.Character Movement`))
  (bind _character_movement_2 (`self.Character Movement`))
  (bind _charactermovement (`Character.CharacterMovement` Character))
  (if (`self.Debug`)
    (`KismetSystemLibrary.PrintString` "Unstick to wall"))
  (set `self.Wall` Wall)
  (set `self.Character Movement` _charactermovement)
  (set `CharacterMovementComponent.bMaintainHorizontalGroundVelocity` false _charactermovement)
  (set `self.IsWallRunning` false)
  (set `CharacterMovementComponent.GravityScale` 2.0 _character_movement_2)
  (set `CharacterMovementComponent.JumpZVelocity` 600.0 _character_movement_2)
  (`MovementComponent.SetPlaneConstraintNormal` _character_movement (0.0 0.0 0.0))
  (set `CharacterMovementComponent.MaxWalkSpeed` (`self.InitialMaxSpeed`) _character_movement))